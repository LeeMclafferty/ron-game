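; BP_Stove is a stove actor whose fire mesh turns like a billboard to follow the player camera.
; Every Tick, GetAngle flattens the camera-to-fire vector onto the horizontal plane and sets FireMesh's world rotation from it, so the mesh only yaws.
; A looping timer alternative exists but is disconnected, and a note marks GetAngle for a move to C++.
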(event EventBeginPlay)

(event EventTick
  (params (DeltaSeconds :type Float%20%28single-precision%29))
  (CallFunction|GetAngle))

(fn ConstructionScript)

(fn GetAngle
  (bind _firemesh (Variables|Default|GetFireMesh))
  ;[1 1 1] Need to move this to CPP
  (Transformation|SetWorldRotation _firemesh (Math|Conversions|RotationFromXVector (Math|Vector|Normalize (* (- (Transformation|GetWorldLocation _firemesh) (Transformation|GetActorLocation (Game|GetPlayerCameraManager 0))) "1.000000,1.000000,0.000000"))) false false))